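; BP_InteractActor is an interactable static-mesh object that an interactor can pick up and drop with pickup presses.
; A press stores the interactor, disables mesh physics, snaps the mesh to the scene root and attaches to the interactor.
; A repeat press by that interactor clears the reference and re-enables physics, with no explicit detach.
; Closest-point queries use mesh collision; other interaction callbacks and events are empty stubs.
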(fn `GetClosestComponentData`
  (params (Interactor :type "/Game/necessary_folder/Blueprints/Components/BPC_WorldInteractor Object Reference"))
  (returns (Point :type "Vector Structure") (Priority :type Integer) (Component :type "SceneComponent Object Reference"))
  (return (`PrimitiveComponent.GetClosestPointOnCollision` (`self.StaticMesh`) (`SceneComponent.K2_GetComponentLocation` Interactor) "None") 0 (`self.StaticMesh`)))

(fn `OnDrag`
  (params (Interactor :type "/Game/necessary_folder/Blueprints/Components/BPC_WorldInteractor Object Reference"))
  (returns (Return :type Boolean))
  (return false))

(fn `OnDragStart`
  (params (Interactor :type "/Game/necessary_folder/Blueprints/Components/BPC_WorldInteractor Object Reference"))
  (returns (Return :type Boolean))
  (return false))

(fn `OnDragStop`
  (params (Interactor :type "/Game/necessary_folder/Blueprints/Components/BPC_WorldInteractor Object Reference"))
  (returns (Return :type Boolean))
  (return false))

(fn `OnHover`
  (params (Interactor :type "/Game/necessary_folder/Blueprints/Components/BPC_WorldInteractor Object Reference"))
  (returns (Return :type Boolean))
  (return false))

(fn `OnHoveredComponentChanged`
  (params (Interactor :type "/Game/necessary_folder/Blueprints/Components/BPC_WorldInteractor Object Reference") (OldComponent :type "SceneComponent Object Reference") (NewComponent :type "SceneComponent Object Reference"))
  (returns (Return :type Boolean))
  (return false))

(fn `OnPickupPressed`
  (params (Interactor :type "/Game/necessary_folder/Blueprints/Components/BPC_WorldInteractor Object Reference"))
  (returns (Return :type Boolean))
  (bind _staticmesh (`self.StaticMesh`))
  (if (and (== (`self.Interator`) Interactor) (`KismetSystemLibrary.IsValid` (`self.Interator`)))
    (set `self.Interator` null)
    (`PrimitiveComponent.SetSimulatePhysics` (`self.StaticMesh`) true)
    (else
      (set `self.Interator` Interactor)
      (`PrimitiveComponent.SetSimulatePhysics` _staticmesh false)
      (`SceneComponent.K2_AttachToComponent` _staticmesh (`self.DefaultSceneRoot`) "None" "SnapToTarget" "SnapToTarget" "KeepWorld" true)
      (`self.K2_AttachToComponent` (`self.Interator`) "None" "SnapToTarget" "SnapToTarget" "KeepWorld")))
  (return false))

(fn `OnPickupReleased`
  (params (Interactor :type "/Game/necessary_folder/Blueprints/Components/BPC_WorldInteractor Object Reference"))
  (returns (Return :type Boolean))
  (return false))

(fn `OnUnhover`
  (params (Interactor :type "/Game/necessary_folder/Blueprints/Components/BPC_WorldInteractor Object Reference"))
  (returns (Return :type Boolean))
  (return false))

(fn `OnUsePressed`
  (params (Interactor :type "/Game/necessary_folder/Blueprints/Components/BPC_WorldInteractor Object Reference"))
  (returns (Return :type Boolean))
  (return false))

(fn `OnUseReleased`
  (params (Interactor :type "/Game/necessary_folder/Blueprints/Components/BPC_WorldInteractor Object Reference"))
  (returns (Return :type Boolean))
  (return false))

(fn `UserConstructionScript`)