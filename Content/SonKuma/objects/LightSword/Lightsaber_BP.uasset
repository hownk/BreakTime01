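; VR lightsaber actor that can be picked up by a hand interactor and switches its blade on and off.
; OnPickupPressed toggles between attaching to the interactor with haptic feedback and dropping with physics restored, calling LSOnOff either way.
; LSOn_off uses a FlipFlop to apply SaberColor and play or reverse a timeline that scales the blade's length, updating light and blade visibility when finished.
; Other interaction handlers, apart from the closest-point query, are stubs returning false.
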(event `self.ReceiveBeginPlay`)

(event `LS On_off`
  (bind _lightblade (`self.Lightblade`))
  (bind _pointlight (`self.PointLight`))
  ;[1 0.7546 0.6676] Lightsaber
  (if false
    (set `self.SaberOut` false :!label _label)
    (bind (_direction _size) (`Timeline|Timeline_0` :!via `ReverseFromEnd` :!label _label_2)
      (:`Update`
        (`SceneComponent.SetWorldScale3D` _lightblade (`KismetMathLibrary.MakeVector` _size 1.0 1.0)))
      (:`Finished`
        (if (`self.SaberOut`)
          (`SceneComponent.SetVisibility` _pointlight true false)
          (else
            (`SceneComponent.SetVisibility` _pointlight false false)
            (`SceneComponent.SetVisibility` _lightblade false false)))))
    (else
      (set `self.Lightsaber R Hand` false)
      (`/Engine/EditorBlueprintResources/StandardMacros.FlipFlop`
        (:`A`
          (`LightComponent.SetLightColor` (`self.PointLight`) (`self.Saber_Color`) true)
          (`PrimitiveComponent.SetMaterial` (`self.Lightblade`) 0 null)
          (`KismetMaterialLibrary.SetVectorParameterValue` null "Blade_Color" (`self.Saber_Color`))
          (set `self.SaberOut` true)
          (`SceneComponent.SetVisibility` _lightblade true false)
          (goto _label_2 :!via `PlayFromStart`))
        (:`B`
          (goto _label))))))

(fn `GetClosestComponentData`
  (params (Interactor :type "/Game/necessary_folder/Blueprints/Components/BPC_WorldInteractor Object Reference"))
  (returns (Point :type "Vector Structure") (Priority :type Integer) (Component :type "SceneComponent Object Reference"))
  (bind _staticmesh (`self.StaticMesh`))
  (return (`PrimitiveComponent.GetClosestPointOnCollision` _staticmesh (`SceneComponent.K2_GetComponentLocation` Interactor) "None") 0 _staticmesh))

(fn `OnDrag`
  (params (Interactor :type "/Game/necessary_folder/Blueprints/Components/BPC_WorldInteractor Object Reference"))
  (returns (Return :type Boolean))
  (return false))

(fn `OnDragStart`
  (params (Interactor :type "/Game/necessary_folder/Blueprints/Components/BPC_WorldInteractor Object Reference"))
  (returns (Return :type Boolean))
  (return false))

(fn `OnDragStop`
  (params (Interactor :type "/Game/necessary_folder/Blueprints/Components/BPC_WorldInteractor Object Reference"))
  (returns (Return :type Boolean))
  (return false))

(fn `OnHover`
  (params (Interactor :type "/Game/necessary_folder/Blueprints/Components/BPC_WorldInteractor Object Reference"))
  (returns (Return :type Boolean))
  (return false))

(fn `OnHoveredComponentChanged`
  (params (Interactor :type "/Game/necessary_folder/Blueprints/Components/BPC_WorldInteractor Object Reference") (OldComponent :type "SceneComponent Object Reference") (NewComponent :type "SceneComponent Object Reference"))
  (returns (Return :type Boolean))
  (return false))

(fn `OnPickupPressed`
  (params (Interactor :type "/Game/necessary_folder/Blueprints/Components/BPC_WorldInteractor Object Reference"))
  (returns (Return :type Boolean))
  (bind _staticmesh (`self.StaticMesh`))
  (bind _interacter (`self.Interacter`))
  (if (and (== _interacter Interactor) (`KismetSystemLibrary.IsValid` _interacter))
    ;[1 1 1] Drop
    (set `self.Interacter` null)
    (`PrimitiveComponent.SetSimulatePhysics` (`self.StaticMesh`) true)
    (else
      ;[1 1 1] Pickup
      (set `self.Interacter` Interactor)
      (`PrimitiveComponent.SetSimulatePhysics` _staticmesh false)
      (`self.K2_SetActorRelativeRotation` (struct :`Yaw` 180.0 :`Roll` 180.0))
      (`SceneComponent.K2_AttachToComponent` _staticmesh (`self.Scene`) "None" "SnapToTarget" "SnapToTarget" "KeepWorld" true)
      (`self.K2_AttachToComponent` (`self.Interacter`) "None" "SnapToTarget" "SnapToTarget" "KeepWorld")
      (`/Game/necessary_folder/Blueprints/FunctionLibraries/BPFL_FeedbackFunctionLibrary.PlayFeedbackOnHand` (`/Game/necessary_folder/Blueprints/Components/BPC_WorldInteractor.GetHand` (`self.Interacter`)) "NewEnumerator0" "NewEnumerator0" (`GameplayStatics.GetPlayerController` 0))))
  (`self.LS On_off`)
  (return false))

(fn `OnPickupReleased`
  (params (Interactor :type "/Game/necessary_folder/Blueprints/Components/BPC_WorldInteractor Object Reference"))
  (returns (Return :type Boolean))
  (return false))

(fn `OnUnhover`
  (params (Interactor :type "/Game/necessary_folder/Blueprints/Components/BPC_WorldInteractor Object Reference"))
  (returns (Return :type Boolean))
  (return false))

(fn `OnUsePressed`
  (params (Interactor :type "/Game/necessary_folder/Blueprints/Components/BPC_WorldInteractor Object Reference"))
  (returns (Return :type Boolean))
  (return false))

(fn `OnUseReleased`
  (params (Interactor :type "/Game/necessary_folder/Blueprints/Components/BPC_WorldInteractor Object Reference"))
  (returns (Return :type Boolean))
  (return false))

(fn `UserConstructionScript`)