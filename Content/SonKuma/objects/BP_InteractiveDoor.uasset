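; Interactive hinged door that an interactor grabs by the handle and swings within yaw limits, with a handle highlight toggled on hover.
; Dragging derives yaw from the interactor's local-space angle around the pivot, minus the grab offset.
; On release, a gated Tick coasts the door from its last yaw speed using closed-form friction deceleration, until it stops or nears a limit.
; CloseDoor plays a timeline back to the initial rotation, ignoring drags meanwhile.
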(event `CloseDoor`
  (set `self.ResettingRotation` true)
  (set `self.InterpDoorRotation` (`SceneComponent.RelativeRotation` (`self.DoorRotate`)))
  (bind (_direction _alpha) (`Timeline|ResetRotationTimeline` :!via `PlayFromStart`)
    (:`Update`
      (`SceneComponent.K2_SetRelativeRotation` (`self.DoorRotate`) (`KismetMathLibrary.RLerp` (`self.InterpDoorRotation`) (`self.InitialDoorRotation`) _alpha) false false))
    (:`Finished`
      (set `self.ResettingRotation` false))))

(event `self.ReceiveBeginPlay`
  (set `self.InitialDoorRotation` (`SceneComponent.RelativeRotation` (`self.DoorRotate`))))

(event `self.ReceiveTick`
  (params (DeltaSeconds :type "Float (single-precision)"))
  (bind _maxyaw (`self.MaxYaw`))
  (bind _minyaw (`self.MinYaw`))
  (bind (_relativerotation_roll _relativerotation_pitch _relativerotation_yaw) (`KismetMathLibrary.BreakRotator` (`SceneComponent.RelativeRotation` (`self.DoorRotate`))))
  (bind _returnvalue (- (`self.DoorInitialYawVelocity`) (* (* (`self.DoorFriction`) 980.0) (`self.DoorTimeSinceLetGo`) (`KismetMathLibrary.SignOfFloat` (`self.DoorInitialYawVelocity`)))))
  (`/Engine/EditorBlueprintResources/StandardMacros.Gate` true :!label _label
    (:`Exit`
      (set `self.DoorTimeSinceLetGo` (+ (`self.DoorTimeSinceLetGo`) DeltaSeconds))
      (if (or (select `bool` (<= (`self.DoorInitialYawVelocity`) 0.0) :`false` (<= _returnvalue 0.0) :`true` (> _returnvalue 0.0)) (>= _relativerotation_yaw _maxyaw) (<= _relativerotation_yaw _minyaw) (`KismetMathLibrary.NearlyEqual_FloatFloat` _relativerotation_yaw _maxyaw 1.0) (`KismetMathLibrary.NearlyEqual_FloatFloat` _minyaw _relativerotation_yaw 1.0))
        (`self.StopSimulateDoorPhysics`)
        (else
          (`SceneComponent.K2_SetRelativeRotation` (`self.DoorRotate`) (`KismetMathLibrary.MakeRotator` 0.0 0.0 (`KismetMathLibrary.ClampAngle` (+ (`self.PhysicsInitialYawAngle`) (- (* (`self.DoorInitialYawVelocity`) (`self.DoorTimeSinceLetGo`)) (* 0.5 (* (`self.DoorFriction`) 980.0) (`KismetMathLibrary.Square` (`self.DoorTimeSinceLetGo`)) (`KismetMathLibrary.SignOfFloat` (`self.DoorInitialYawVelocity`))))) (`self.MinYaw`) (`self.MaxYaw`))) false false))))))

(event `StartSimulateDoorPhysics`
  (params (InitialYawVelocity :type "Float (double-precision)"))
  (bind (_relativerotation_roll _relativerotation_pitch _relativerotation_yaw) (`KismetMathLibrary.BreakRotator` (`SceneComponent.RelativeRotation` (`self.DoorRotate`))))
  (set `self.DoorInitialYawVelocity` InitialYawVelocity)
  (set `self.PhysicsInitialYawAngle` _relativerotation_yaw)
  (set `self.DoorTimeSinceLetGo` 0.0)
  (goto _label :!via `Open`))

(event `StopSimulateDoorPhysics`
  (goto _label :!via `Close`))

(fn `GetClosestComponentData`
  (params (Interactor :type "/Game/necessary_folder/Blueprints/Components/BPC_WorldInteractor Object Reference"))
  (returns (Point :type "Vector Structure") (Priority :type Integer) (Component :type "SceneComponent Object Reference"))
  (return (`PrimitiveComponent.GetClosestPointOnCollision` (`self.DoorHandle`) (`SceneComponent.K2_GetComponentLocation` Interactor) "None") 0 (`self.DoorHandle`)))

(fn `OnDrag`
  (params (Interactor :type "/Game/necessary_folder/Blueprints/Components/BPC_WorldInteractor Object Reference"))
  (returns (Return :type Boolean))
  (bind _output_get (set `self.CurrentInteractor` Interactor))
  (if (not (`self.ResettingRotation`))
    (set `self.PreviousRotation` (`SceneComponent.RelativeRotation` (`self.DoorRotate`)))
    (bind (_returnvalue_x _returnvalue_y) (`KismetMathLibrary.BreakVector` (- (`KismetMathLibrary.InverseTransformLocation` (`self.GetTransform`) (`SceneComponent.K2_GetComponentLocation` _output_get)) (`SceneComponent.RelativeLocation` (`self.DoorRotate`)))))
    (`SceneComponent.K2_SetRelativeRotation` (`self.DoorRotate`) (`KismetMathLibrary.MakeRotator` 0.0 0.0 (`KismetMathLibrary.ClampAngle` (- (`KismetMathLibrary.DegAtan2` _returnvalue_y _returnvalue_x) (`self.DoorInitialGrabOffset`)) (`self.MinYaw`) (`self.MaxYaw`))) false false)
    (return true)
    (else
      (return false))))

(fn `OnDragStart`
  (params (Interactor :type "/Game/necessary_folder/Blueprints/Components/BPC_WorldInteractor Object Reference"))
  (returns (Return :type Boolean))
  (bind (_relativerotation_roll _relativerotation_pitch _relativerotation_yaw) (`KismetMathLibrary.BreakRotator` (`SceneComponent.RelativeRotation` (`self.DoorRotate`))))
  (bind (_returnvalue_x _returnvalue_y) (`KismetMathLibrary.BreakVector` (- (`KismetMathLibrary.InverseTransformLocation` (`self.GetTransform`) (`SceneComponent.K2_GetComponentLocation` Interactor)) (`SceneComponent.RelativeLocation` (`self.DoorRotate`)))))
  (set `self.DoorInitialGrabOffset` (- (`KismetMathLibrary.DegAtan2` _returnvalue_y _returnvalue_x) _relativerotation_yaw))
  (`self.StopSimulateDoorPhysics`)
  (return false))

(fn `OnDragStop`
  (params (Interactor :type "/Game/necessary_folder/Blueprints/Components/BPC_WorldInteractor Object Reference"))
  (returns (Return :type Boolean))
  (bind (_previousrotation_roll _previousrotation_pitch _previousrotation_yaw) (`KismetMathLibrary.BreakRotator` (`self.PreviousRotation`)))
  (bind (_relativerotation_roll _relativerotation_pitch _relativerotation_yaw) (`KismetMathLibrary.BreakRotator` (`SceneComponent.RelativeRotation` (`self.DoorRotate`))))
  (`self.StartSimulateDoorPhysics` (/ (- _relativerotation_yaw _previousrotation_yaw) (`GameplayStatics.GetWorldDeltaSeconds`)))
  (return false))

(fn `OnHover`
  (params (Interactor :type "/Game/necessary_folder/Blueprints/Components/BPC_WorldInteractor Object Reference"))
  (returns (Return :type Boolean))
  (`SceneComponent.ToggleVisibility` (`self.DoorHandleHighlighted`) false)
  (return false))

(fn `OnHoveredComponentChanged`
  (params (Interactor :type "/Game/necessary_folder/Blueprints/Components/BPC_WorldInteractor Object Reference") (OldComponent :type "SceneComponent Object Reference") (NewComponent :type "SceneComponent Object Reference"))
  (returns (Return :type Boolean))
  (return false))

(fn `OnPickupPressed`
  (params (Interactor :type "/Game/necessary_folder/Blueprints/Components/BPC_WorldInteractor Object Reference"))
  (returns (Return :type Boolean))
  (return false))

(fn `OnPickupReleased`
  (params (Interactor :type "/Game/necessary_folder/Blueprints/Components/BPC_WorldInteractor Object Reference"))
  (returns (Return :type Boolean))
  (return false))

(fn `OnUnhover`
  (params (Interactor :type "/Game/necessary_folder/Blueprints/Components/BPC_WorldInteractor Object Reference"))
  (returns (Return :type Boolean))
  (`SceneComponent.ToggleVisibility` (`self.DoorHandleHighlighted`) false)
  (return false))

(fn `OnUsePressed`
  (params (Interactor :type "/Game/necessary_folder/Blueprints/Components/BPC_WorldInteractor Object Reference"))
  (returns (Return :type Boolean))
  (return false))

(fn `OnUseReleased`
  (params (Interactor :type "/Game/necessary_folder/Blueprints/Components/BPC_WorldInteractor Object Reference"))
  (returns (Return :type Boolean))
  (return false))

(fn `UserConstructionScript`)