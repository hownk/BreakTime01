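; BP_Climbactor is a ladder-folder interactable, apparently meant as a climbable grab target, though no climbing movement is implemented here.
; It reports the closest collision point on its static mesh to the Interactor, at priority zero.
; Pickup press stores the Interactor, but the node that clears it is unconnected, so release never resets it.
; The other hover, drag, use and release handlers are stubs returning false.
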(fn `GetClosestComponentData`
  (params (Interactor :type "/Game/necessary_folder/Blueprints/Components/BPC_WorldInteractor Object Reference"))
  (returns (Point :type "Vector Structure") (Priority :type Integer) (Component :type "SceneComponent Object Reference"))
  (bind _staticmeshcomponent (`self.StaticMeshComponent`))
  (return (`PrimitiveComponent.GetClosestPointOnCollision` _staticmeshcomponent (`SceneComponent.K2_GetComponentLocation` Interactor) "None") 0 _staticmeshcomponent))

(fn `OnDrag`
  (params (Interactor :type "/Game/necessary_folder/Blueprints/Components/BPC_WorldInteractor Object Reference"))
  (returns (Return :type Boolean))
  (return false))

(fn `OnDragStart`
  (params (Interactor :type "/Game/necessary_folder/Blueprints/Components/BPC_WorldInteractor Object Reference"))
  (returns (Return :type Boolean))
  (return false))

(fn `OnDragStop`
  (params (Interactor :type "/Game/necessary_folder/Blueprints/Components/BPC_WorldInteractor Object Reference"))
  (returns (Return :type Boolean))
  (return false))

(fn `OnHover`
  (params (Interactor :type "/Game/necessary_folder/Blueprints/Components/BPC_WorldInteractor Object Reference"))
  (returns (Return :type Boolean))
  (return false))

(fn `OnHoveredComponentChanged`
  (params (Interactor :type "/Game/necessary_folder/Blueprints/Components/BPC_WorldInteractor Object Reference") (OldComponent :type "SceneComponent Object Reference") (NewComponent :type "SceneComponent Object Reference"))
  (returns (Return :type Boolean))
  (return false))

(fn `OnPickupPressed`
  (params (Interactor :type "/Game/necessary_folder/Blueprints/Components/BPC_WorldInteractor Object Reference"))
  (returns (Return :type Boolean))
  (`/Engine/EditorBlueprintResources/StandardMacros.IsValid` (`self.Interactor`)
    (:`Is Valid`
      (if (not (== (`self.Interactor`) Interactor))
        (set `self.Interactor` Interactor :!label _label)))
    (:`Is Not Valid`
      (goto _label))))

(fn `OnPickupReleased`
  (params (Interactor :type "/Game/necessary_folder/Blueprints/Components/BPC_WorldInteractor Object Reference"))
  (returns (Return :type Boolean))
  (return false))

(fn `OnUnhover`
  (params (Interactor :type "/Game/necessary_folder/Blueprints/Components/BPC_WorldInteractor Object Reference"))
  (returns (Return :type Boolean))
  (return false))

(fn `OnUsePressed`
  (params (Interactor :type "/Game/necessary_folder/Blueprints/Components/BPC_WorldInteractor Object Reference"))
  (returns (Return :type Boolean))
  (return false))

(fn `OnUseReleased`
  (params (Interactor :type "/Game/necessary_folder/Blueprints/Components/BPC_WorldInteractor Object Reference"))
  (returns (Return :type Boolean))
  (return false))

(fn `UserConstructionScript`)