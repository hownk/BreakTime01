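; BP_Eraser is a hand-held whiteboard eraser that can be picked up and clears the BP_WhiteBoard it touches.
; Pickup presses attach it to the interactor or release it to physics, while Front overlaps set the target board and trigger hand feedback.
; Each tick, it intersects the twelve edges of its rotated Box with the board plane and draws that cross-section as a polygon using a clear material.
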(event `self.ReceiveTick`
  (params (DeltaSeconds :type "Float (single-precision)"))
  (`/Engine/EditorBlueprintResources/StandardMacros.IsValid` (`self.Whiteboard`)
    (:`Is Valid`
      (bind _out (`self.GetIntersectionVertices`))
      (`/Game/SonKuma/objects/BP_WhiteBoard.DrawPolygon` (`self.Whiteboard`) _out "/Game/necessary_folder/Materials/M_WhiteBoardClearMaterial.M_WhiteBoardClearMaterial"))))

(event `self.Front.OnComponentBeginOverlap`
  (params (OverlappedComponent :type "PrimitiveComponent Object Reference") (OtherActor :type "Actor Object Reference") (OtherComp :type "PrimitiveComponent Object Reference") (OtherBodyIndex :type Integer) (bFromSweep :type Boolean) (SweepResult :type "HitResult Structure (by ref)"))
  (bind _interactor (`self.Interactor`))
  (bind _asbp_white_board (cast `/Game/SonKuma/objects/BP_WhiteBoard` OtherActor))
  (set `self.Whiteboard` _asbp_white_board)
  (`/Engine/EditorBlueprintResources/StandardMacros.IsValid` _interactor
    (:`Is Valid`
      (`/Game/necessary_folder/Blueprints/FunctionLibraries/BPFL_FeedbackFunctionLibrary.PlayFeedbackOnHand` (`/Game/necessary_folder/Blueprints/Components/BPC_WorldInteractor.GetHand` _interactor) "NewEnumerator0" "NewEnumerator0" (`GameplayStatics.GetPlayerController` 0)))))

(event `self.Front.OnComponentEndOverlap`
  (params (OverlappedComponent :type "PrimitiveComponent Object Reference") (OtherActor :type "Actor Object Reference") (OtherComp :type "PrimitiveComponent Object Reference") (OtherBodyIndex :type Integer))
  (if (== OtherActor (`self.Whiteboard`))
    (set `self.Whiteboard` null)))

(fn `GetBoxVerts`
  (params (Origin :type "Vector Structure") (Extent :type "Vector Structure") (Rotation :type "Rotator Structure"))
  (returns (Vertices :type "Array of Vector Structure") (Edges :type "Array of Integer"))
  (locals (InOrigin :type "Vector Structure") (InExtent :type "Vector Structure") (InRotation :type "Rotator Structure") (tmpVertices :type "Array of Vector Structure") (tmpEdges :type "Array of Integer"))
  (bind (_inextent_x _inextent_y _inextent_z) (`KismetMathLibrary.BreakVector` (`local.InExtent`)))
  (bind (_inextent_x_2 _inextent_y_2 _inextent_z_2) (`KismetMathLibrary.BreakVector` (`local.InExtent`)))
  (bind (_inextent_x_3 _inextent_y_3 _inextent_z_3) (`KismetMathLibrary.BreakVector` (`local.InExtent`)))
  (bind (_inextent_x_4 _inextent_y_4 _inextent_z_4) (`KismetMathLibrary.BreakVector` (`local.InExtent`)))
  (bind (_inextent_x_5 _inextent_y_5 _inextent_z_5) (`KismetMathLibrary.BreakVector` (`local.InExtent`)))
  (bind (_inextent_x_6 _inextent_y_6 _inextent_z_6) (`KismetMathLibrary.BreakVector` (`local.InExtent`)))
  (set `local.InOrigin` Origin)
  (set `local.InExtent` Extent)
  (set `local.InRotation` Rotation)
  (set `local.tmpVertices` (`|MakeArray` (+ (`local.InOrigin`) (`KismetMathLibrary.GreaterGreater_VectorRotator` (`local.InExtent`) (`local.InRotation`))) (- (`local.InOrigin`) (`KismetMathLibrary.GreaterGreater_VectorRotator` (`local.InExtent`) (`local.InRotation`))) (+ (`local.InOrigin`) (`KismetMathLibrary.GreaterGreater_VectorRotator` (`KismetMathLibrary.MakeVector` (* _inextent_x -1.0) _inextent_y _inextent_z) (`local.InRotation`))) (+ (`local.InOrigin`) (`KismetMathLibrary.GreaterGreater_VectorRotator` (`KismetMathLibrary.MakeVector` _inextent_x_2 (* _inextent_y_2 -1.0) _inextent_z_2) (`local.InRotation`))) (+ (`local.InOrigin`) (`KismetMathLibrary.GreaterGreater_VectorRotator` (`KismetMathLibrary.MakeVector` _inextent_x_3 _inextent_y_3 (* _inextent_z_3 -1.0)) (`local.InRotation`))) (+ (`local.InOrigin`) (`KismetMathLibrary.GreaterGreater_VectorRotator` (`KismetMathLibrary.MakeVector` (* _inextent_x_4 -1.0) (* _inextent_y_4 -1.0) _inextent_z_4) (`local.InRotation`))) (+ (`local.InOrigin`) (`KismetMathLibrary.GreaterGreater_VectorRotator` (`KismetMathLibrary.MakeVector` _inextent_x_5 (* _inextent_y_5 -1.0) (* _inextent_z_5 -1.0)) (`local.InRotation`))) (+ (`local.InOrigin`) (`KismetMathLibrary.GreaterGreater_VectorRotator` (`KismetMathLibrary.MakeVector` (* _inextent_x_6 -1.0) _inextent_y_6 (* _inextent_z_6 -1.0)) (`local.InRotation`)))))
  ;[1 1 1] Manually create edges for these vertices
  (set `local.tmpEdges` (`|MakeArray` 0 3 0 4 0 2 6 3 6 4 6 1 3 5 4 7 2 7 2 5 1 5 1 7))
  (return (`local.tmpVertices`) (`local.tmpEdges`)))

(fn `GetClosestComponentData`
  (params (Interactor :type "/Game/necessary_folder/Blueprints/Components/BPC_WorldInteractor Object Reference"))
  (returns (Point :type "Vector Structure") (Priority :type Integer) (Component :type "SceneComponent Object Reference"))
  (return (`PrimitiveComponent.GetClosestPointOnCollision` (`self.Back`) (`SceneComponent.K2_GetComponentLocation` Interactor) "None") 0 (`self.Back`)))

(fn `GetIntersectionVertices`
  (returns (Out :type "Array of Vector Structure"))
  (locals (BoxVerts :type "Array of Vector Structure") (BoxEdges :type "Array of Integer") (IntersectionVerts :type "Array of Vector Structure"))
  (bind _box (`self.Box`))
  (bind _board (`/Game/SonKuma/objects/BP_WhiteBoard.Board` (`self.Whiteboard`)))
  (bind (_vertices _edges) (`self.GetBoxVerts` (`SceneComponent.K2_GetComponentLocation` _box) (`BoxComponent.BoxExtent` _box) (`SceneComponent.K2_GetComponentRotation` (`self.Box`))))
  (set `local.BoxVerts` _vertices)
  (set `local.BoxEdges` _edges)
  (for _index (range 12)
    (bind _returnvalue (* _index 2))
    (bind (_t _intersection _returnvalue_2) (`KismetMathLibrary.LinePlaneIntersection` (`KismetArrayLibrary.Array_Get` (`local.BoxVerts`) (`KismetArrayLibrary.Array_Get` (`local.BoxEdges`) _returnvalue)) (`KismetArrayLibrary.Array_Get` (`local.BoxVerts`) (`KismetArrayLibrary.Array_Get` (`local.BoxEdges`) (+ _returnvalue 1))) (`KismetMathLibrary.MakePlaneFromPointAndNormal` (`SceneComponent.K2_GetComponentLocation` _board) (`SceneComponent.GetForwardVector` _board))))
    (if _returnvalue_2
      (`KismetArrayLibrary.Array_Add` (`local.IntersectionVerts`) _intersection)))
  (return (`local.IntersectionVerts`)))

(fn `OnDrag`
  (params (Interactor :type "/Game/necessary_folder/Blueprints/Components/BPC_WorldInteractor Object Reference"))
  (returns (Return :type Boolean))
  (return false))

(fn `OnDragStart`
  (params (Interactor :type "/Game/necessary_folder/Blueprints/Components/BPC_WorldInteractor Object Reference"))
  (returns (Return :type Boolean))
  (return false))

(fn `OnDragStop`
  (params (Interactor :type "/Game/necessary_folder/Blueprints/Components/BPC_WorldInteractor Object Reference"))
  (returns (Return :type Boolean))
  (return false))

(fn `OnHover`
  (params (Interactor :type "/Game/necessary_folder/Blueprints/Components/BPC_WorldInteractor Object Reference"))
  (returns (Return :type Boolean))
  (return false))

(fn `OnHoveredComponentChanged`
  (params (Interactor :type "/Game/necessary_folder/Blueprints/Components/BPC_WorldInteractor Object Reference") (OldComponent :type "SceneComponent Object Reference") (NewComponent :type "SceneComponent Object Reference"))
  (returns (Return :type Boolean))
  (return false))

(fn `OnPickupPressed`
  (params (Interactor :type "/Game/necessary_folder/Blueprints/Components/BPC_WorldInteractor Object Reference"))
  (returns (Return :type Boolean))
  (bind _back (`self.Back`))
  (`/Engine/EditorBlueprintResources/StandardMacros.IsValid` (`self.Interactor`)
    (:`Is Valid`
      (if (== (`self.Interactor`) Interactor)
        (`PrimitiveComponent.SetSimulatePhysics` (`self.Back`) true)
        (set `self.Interactor` null)
        (else
          (set `self.Interactor` Interactor :!label _label)
          (`PrimitiveComponent.SetSimulatePhysics` _back false)
          (`SceneComponent.K2_AttachToComponent` _back (`self.EraserRoot`) "None" "SnapToTarget" "SnapToTarget" "KeepWorld" true)
          (`self.K2_AttachToComponent` (`self.Interactor`) "None" "SnapToTarget" "SnapToTarget" "KeepWorld"))))
    (:`Is Not Valid`
      (goto _label)))
  (return false))

(fn `OnPickupReleased`
  (params (Interactor :type "/Game/necessary_folder/Blueprints/Components/BPC_WorldInteractor Object Reference"))
  (returns (Return :type Boolean))
  (return false))

(fn `OnUnhover`
  (params (Interactor :type "/Game/necessary_folder/Blueprints/Components/BPC_WorldInteractor Object Reference"))
  (returns (Return :type Boolean))
  (return false))

(fn `OnUsePressed`
  (params (Interactor :type "/Game/necessary_folder/Blueprints/Components/BPC_WorldInteractor Object Reference"))
  (returns (Return :type Boolean))
  (return false))

(fn `OnUseReleased`
  (params (Interactor :type "/Game/necessary_folder/Blueprints/Components/BPC_WorldInteractor Object Reference"))
  (returns (Return :type Boolean))
  (return false))

(fn `UserConstructionScript`)