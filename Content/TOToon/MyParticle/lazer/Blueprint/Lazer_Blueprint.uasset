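; Lazer_Blueprint is a configurable laser effect actor that pairs a particle system with a RotatingMovement component.
; The Construction Script copies the actor's pivot translation, rotation rate and local-space setting into the rotating movement.
; It also passes the color and alpha variables to the particle system's TOTColor and TOTAlpha parameters.
; The Event Graph holds no logic, so all setup happens at construction.
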(fn `UserConstructionScript`
  (bind _particlesystemcomponent (`self.ParticleSystemComponent`))
  (bind _rotatingmovement (`self.RotatingMovement`))
  (set `RotatingMovementComponent.PivotTranslation` (`self.Pivot Translation`) _rotatingmovement)
  (set `RotatingMovementComponent.RotationRate` (`self.Rotation Rate`) _rotatingmovement)
  (set `RotatingMovementComponent.bRotationInLocalSpace` (`self.Rotation in Local Space`) _rotatingmovement)
  (`ParticleSystemComponent.SetVectorParameter` _particlesystemcomponent "TOTColor" (`self.Particle Color`))
  (`ParticleSystemComponent.SetFloatParameter` _particlesystemcomponent "TOTAlpha" (`self.Set Alpha`)))