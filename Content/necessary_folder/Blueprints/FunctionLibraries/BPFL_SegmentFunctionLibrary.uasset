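; Blueprint function library of search helpers for arrays of segments, each compared by its Value field.
; FindMinMax returns the segments with the lowest and highest values.
; FindSegmentWithValue returns the first segment within a threshold of a target value plus a success flag, while FindClosestSegment returns the one with the smallest absolute difference.
; All use linear loops; the min/max and closest searches seed their result from the first element through DoOnce.
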(fn `FindClosestSegment`
  (params (Value :type "Float (double-precision)") (Segments :type "Array of /Game/necessary_folder/Blueprints/Structs/SSegmentStruct Structure"))
  (returns (ClosestSegment :type "/Game/necessary_folder/Blueprints/Structs/SSegmentStruct Structure"))
  (locals (tmpClosestSegment :type "/Game/necessary_folder/Blueprints/Structs/SSegmentStruct Structure" :default (struct)) (closestSegmentDelta :type "Float (double-precision)" :default "(Value_6_CCECF1F546DE288ED3B216A381CF9076=0.000000,Name_5_93D46F8948F76E8A0F793EAF46D36AFA=)"))
  (for _array_element Segments
    (`|ExecutionSequence`
      (:`then_0`
        (`/Engine/EditorBlueprintResources/StandardMacros.DoOnce` false
          (:`Completed`
            (bind _returnvalue (`KismetMathLibrary.Abs` (- Value (`.Value_6_CCECF1F546DE288ED3B216A381CF9076` (break `/Game/necessary_folder/Blueprints/Structs/SSegmentStruct` _array_element)))))
            (set `local.closestSegmentDelta` _returnvalue)
            (set `local.tmpClosestSegment` _array_element))))
      (:`then_1`
        (if (< _returnvalue (`local.closestSegmentDelta`))
          (set `local.closestSegmentDelta` _returnvalue)
          (set `local.tmpClosestSegment` _array_element)))))
  (return (`local.tmpClosestSegment`)))

(fn `FindMinMax`
  (params (Seqments :type "Array of /Game/necessary_folder/Blueprints/Structs/SSegmentStruct Structure"))
  (returns (Min :type "/Game/necessary_folder/Blueprints/Structs/SSegmentStruct Structure") (Max :type "/Game/necessary_folder/Blueprints/Structs/SSegmentStruct Structure"))
  (locals (tmpMin :type "/Game/necessary_folder/Blueprints/Structs/SSegmentStruct Structure" :default (struct)) (tmpMax :type "/Game/necessary_folder/Blueprints/Structs/SSegmentStruct Structure" :default (struct)))
  (for _array_element Seqments
    (`|ExecutionSequence`
      (:`then_0`
        (`/Engine/EditorBlueprintResources/StandardMacros.DoOnce` false
          (:`Completed`
            (set `local.tmpMin` _array_element)
            (set `local.tmpMax` _array_element))))
      (:`then_1`
        (if (> (`.Value_6_CCECF1F546DE288ED3B216A381CF9076` (break `/Game/necessary_folder/Blueprints/Structs/SSegmentStruct` _array_element)) (`.Value_6_CCECF1F546DE288ED3B216A381CF9076` (break `/Game/necessary_folder/Blueprints/Structs/SSegmentStruct` (`local.tmpMax`))))
          (set `local.tmpMax` _array_element)))
      (:`then_2`
        (if (< (`.Value_6_CCECF1F546DE288ED3B216A381CF9076` (break `/Game/necessary_folder/Blueprints/Structs/SSegmentStruct` _array_element)) (`.Value_6_CCECF1F546DE288ED3B216A381CF9076` (break `/Game/necessary_folder/Blueprints/Structs/SSegmentStruct` (`local.tmpMin`))))
          (set `local.tmpMin` _array_element)))))
  (return (`local.tmpMin`) (`local.tmpMax`)))

(fn `FindSegmentWithValue`
  (params (Value :type "Float (double-precision)") (Threshold :type "Float (double-precision)") (Segments :type "Array of /Game/necessary_folder/Blueprints/Structs/SSegmentStruct Structure"))
  (returns (Segment :type "/Game/necessary_folder/Blueprints/Structs/SSegmentStruct Structure") (Success :type Boolean))
  (locals (tmpSegment :type "/Game/necessary_folder/Blueprints/Structs/SSegmentStruct Structure" :default (struct)) (tmpSuccess :type Boolean :default false))
  (for _array_element Segments
    (bind _value (break `/Game/necessary_folder/Blueprints/Structs/SSegmentStruct` _array_element))
    (if (and (>= _value (- Value Threshold)) (<= _value (+ Value Threshold)))
      (set `local.tmpSegment` _array_element)
      (set `local.tmpSuccess` true)
      (break)))
  (return (`local.tmpSegment`) (`local.tmpSuccess`)))