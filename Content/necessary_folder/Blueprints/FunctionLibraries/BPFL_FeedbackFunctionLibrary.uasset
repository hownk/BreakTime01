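; Blueprint function library that plays controller haptic feedback on a given hand.
; PlayFeedbackOnHand switches on feedback type (Burst or Shake), then on intensity (Low or High), to pick one of four haptic effects.
; The chosen effect plays through the supplied Player Controller's PlayHapticEffect on that hand.
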(fn `PlayFeedbackOnHand`
  (params (Hand :type "EControllerHand Enum") (Type :type "/Game/necessary_folder/Blueprints/FeedbackEffects/EFeedbackType Enum") (Intensity :type "/Game/necessary_folder/Blueprints/FeedbackEffects/EFeedbackIntensity Enum") (PlayerController :type "PlayerController Object Reference"))
  (locals (Scale :type "Float (double-precision)" :default 3.0))
  (switch `/Game/necessary_folder/Blueprints/FeedbackEffects/EFeedbackType` Type
    (:`NewEnumerator0`
      (switch `/Game/necessary_folder/Blueprints/FeedbackEffects/EFeedbackIntensity` Intensity
        (:`NewEnumerator0`
          (`PlayerController.PlayHapticEffect` PlayerController "/Game/necessary_folder/Blueprints/FeedbackEffects/LowIntensityBurst.LowIntensityBurst" Hand (`local.Scale`) false))
        (:`NewEnumerator1`
          (`PlayerController.PlayHapticEffect` PlayerController "/Game/necessary_folder/Blueprints/FeedbackEffects/HighIntensityBurst.HighIntensityBurst" Hand (`local.Scale`) false))))
    (:`NewEnumerator1`
      (switch `/Game/necessary_folder/Blueprints/FeedbackEffects/EFeedbackIntensity` Intensity
        (:`NewEnumerator0`
          (`PlayerController.PlayHapticEffect` PlayerController "/Game/necessary_folder/Blueprints/FeedbackEffects/LowIntensityShake.LowIntensityShake" Hand (`local.Scale`) false))
        (:`NewEnumerator1`
          (`PlayerController.PlayHapticEffect` PlayerController "/Game/necessary_folder/Blueprints/FeedbackEffects/HighIntensityShake.HighIntensityShake" Hand (`local.Scale`) false))))))