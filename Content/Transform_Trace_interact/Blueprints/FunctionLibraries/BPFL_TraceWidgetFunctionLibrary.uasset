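; Function library of UMG helpers for mapping positions onto widgets and gathering their children, apparently for trace-based widget interaction.
; WorldSpaceToWidgetSpace inverse-transforms a world location into widget component space, then flips and offsets it into top-left draw-size coordinates.
; ParentWidgetSpaceToChildSpace offsets a parent position by a canvas slot's position and minimum anchor.
; GetCanvasChildren optionally recurses through nested canvases, while GetPanelChildren always flattens nested panels into leaf widgets.
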(fn `GetCanvasChildren`
  (params (Deep :type Boolean) (Root :type "CanvasPanel Object Reference"))
  (returns (Widgets :type "Array of Widget Object Reference"))
  (locals (tmpChildren :type "Array of Widget Object Reference"))
  ;[1 1 1] Find all children under a canvas panel
  (for _index (range (`PanelWidget.GetChildrenCount` Root))
    (if Deep
      (bind _returnvalue (`PanelWidget.GetChildAt` Root _index))
      (bind _ascanvas_panel (cast `CanvasPanel` _returnvalue)
        (:`then`
          (bind _widgets (`self.GetCanvasChildren` Deep _ascanvas_panel _ascanvas_panel))
          (`KismetArrayLibrary.Array_Append` (`local.tmpChildren`) _widgets))
        (:`CastFailed`
          (`KismetArrayLibrary.Array_Add` (`local.tmpChildren`) _returnvalue :!label _label) ; If shallow search or widget is not a canvas panel
        ))
      (else
        (goto _label))))
  (return (`local.tmpChildren`)))

(fn `GetPanelChildren`
  (params (Panel :type "PanelWidget Object Reference"))
  (returns (Widgets :type "Array of Widget Object Reference"))
  (locals (inPanel :type "PanelWidget Object Reference") (tmpChildren :type "Array of Widget Object Reference"))
  (set `local.inPanel` Panel)
  (for _index (range (`PanelWidget.GetChildrenCount` (`local.inPanel`)))
    (bind _returnvalue (`PanelWidget.GetChildAt` (`local.inPanel`) _index))
    (bind _aspanel_widget (cast `PanelWidget` _returnvalue)
      (:`then`
        (bind _widgets (`self.GetPanelChildren` _aspanel_widget (`local.inPanel`)))
        (`KismetArrayLibrary.Array_Append` (`local.tmpChildren`) _widgets))
      (:`CastFailed`
        (`KismetArrayLibrary.Array_Add` (`local.tmpChildren`) _returnvalue))))
  (return (`local.tmpChildren`)))

(fn `ParentWidgetSpaceToChildSpace`
  (params (Position :type "Vector2D Structure") (ParentSize :type "Vector2D Structure") (ChildSlot :type "CanvasPanelSlot Object Reference"))
  (returns (ReturnValue :type "Vector2D Structure"))
  (bind (_x _y) (`KismetMathLibrary.BreakVector2D` ParentSize))
  (bind (_minimum_x _minimum_y) (`KismetMathLibrary.BreakVector2D` (break `Anchors` (`CanvasPanelSlot.GetAnchors` ChildSlot))))
  (return (- Position (+ (`CanvasPanelSlot.GetPosition` ChildSlot) (`KismetMathLibrary.MakeVector2D` (* _x _minimum_x) (* _y _minimum_y))))))

(fn `WorldSpaceToWidgetSpace`
  (params (Location :type "Vector Structure") (Target :type "WidgetComponent Object Reference"))
  (returns (WidgetPosition :type "Vector2D Structure"))
  (bind (_returnvalue_x _returnvalue_y) (`KismetMathLibrary.BreakVector2D` (`WidgetComponent.GetDrawSize` Target)))
  (return (`KismetMathLibrary.MakeVector2D` (+ (* (.y (`KismetMathLibrary.InverseTransformLocation` (`SceneComponent.K2_GetComponentToWorld` Target) Location)) -1.0) (/ _returnvalue_x 2.0)) (+ (* (.z (`KismetMathLibrary.InverseTransformLocation` (`SceneComponent.K2_GetComponentToWorld` Target) Location)) -1.0) (/ _returnvalue_y 2.0)))))