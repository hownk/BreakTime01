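; BP_TeleportNode is a fixed VR teleport point that the player activates through trace interaction.
; A child BP_TeleportPreview serves as its marker, blue by default with chaperone bounds hidden.
; Trace enter and leave toggle PVRTeleport visibility and switch the marker between green and blue.
; Trace up moves the pawn to the node plus TeleportToLocation, compensating for the horizontal camera-to-pawn offset.
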(event `self.ReceiveBeginPlay`
  (`parent.ReceiveBeginPlay`)
  ;[1 1 1] Get the actual teleport preview
  (bind _asbp_teleport_preview (cast `/Game/Transform_Trace_interact/Blueprints/BP_TeleportPreview` (`ChildActorComponent.ChildActor` (`self.TeleportPreview`))))
  (set `self.TeleportPreviewObject` _asbp_teleport_preview)
  (`self.SetupNode`))

(fn `SetupNode`
  ;[1 1 1] Default color to blue
  (bind _asbp_teleport_preview (cast `/Game/Transform_Trace_interact/Blueprints/BP_TeleportPreview` (`ChildActorComponent.ChildActor` (`self.TeleportPreview`))))
  (`/Game/Transform_Trace_interact/Blueprints/BP_TeleportPreview.SetColor` _asbp_teleport_preview (struct :`R` 0.127647 :`G` 0.59241 :`B` 1.0 :`A` 1.0))
  ;[1 1 1] Don't draw the chaperone bounds on a node
  (`SceneComponent.SetHiddenInGame` (`/Game/Transform_Trace_interact/Blueprints/BP_TeleportPreview.TeleportChaperoneBounds` _asbp_teleport_preview) true false))

(fn `ShouldInteractWithWidgets`
  (returns (Return :type Boolean))
  (return false))

(fn `TeleportPlayer`
  (bind (_returnvalue_x _returnvalue_y) (`KismetMathLibrary.BreakVector` (- (`self.K2_GetActorLocation` (`GameplayStatics.GetPlayerPawn` 0)) (`PlayerCameraManager.GetCameraLocation` (`GameplayStatics.GetPlayerCameraManager` 0)))))
  (`self.K2_SetActorLocation` (`GameplayStatics.GetPlayerPawn` 0) (+ (+ (`self.K2_GetActorLocation`) (`self.TeleportToLocation`)) (`KismetMathLibrary.MakeVector` _returnvalue_x _returnvalue_y)) false false))

(fn `TraceDown`
  (params (Hit :type "HitResult Structure") (Interactor :type "/Game/Transform_Trace_interact/Blueprints/Components/BP_TraceInteractor Object Reference"))
  (returns (Return :type Boolean))
  (return false))

(fn `TraceEnter`
  (params (Hit :type "HitResult Structure") (Interactor :type "/Game/Transform_Trace_interact/Blueprints/Components/BP_TraceInteractor Object Reference"))
  (returns (Return :type Boolean))
  (`SceneComponent.SetVisibility` (`self.P_VRTeleport`) true false)
  (`/Game/Transform_Trace_interact/Blueprints/BP_TeleportPreview.SetColor` (`self.TeleportPreviewObject`) (struct :`R` 0.249933 :`G` 1.0 :`B` 0.464466 :`A` 1.0))
  (return false))

(fn `TraceLeave`
  (params (Hit :type "HitResult Structure") (Interactor :type "/Game/Transform_Trace_interact/Blueprints/Components/BP_TraceInteractor Object Reference"))
  (returns (Return :type Boolean))
  (`SceneComponent.SetVisibility` (`self.P_VRTeleport`) false false)
  (`/Game/Transform_Trace_interact/Blueprints/BP_TeleportPreview.SetColor` (`self.TeleportPreviewObject`) (struct :`R` 0.127647 :`G` 0.59241 :`B` 1.0 :`A` 1.0))
  (return false))

(fn `TraceMove`
  (params (Hit :type "HitResult Structure (by ref)") (Interactor :type "/Game/Transform_Trace_interact/Blueprints/Components/BP_TraceInteractor Object Reference"))
  (returns (Return :type Boolean))
  (return false))

(fn `TraceOut`
  (params (Hit :type "HitResult Structure") (Interactor :type "/Game/Transform_Trace_interact/Blueprints/Components/BP_TraceInteractor Object Reference") (LeavingComponent :type "PrimitiveComponent Object Reference"))
  (returns (Return :type Boolean))
  (return false))

(fn `TraceOver`
  (params (Hit :type "HitResult Structure") (Interactor :type "/Game/Transform_Trace_interact/Blueprints/Components/BP_TraceInteractor Object Reference") (HitComponent :type "PrimitiveComponent Object Reference"))
  (returns (Return :type Boolean))
  (return false))

(fn `TraceUp`
  (params (Hit :type "HitResult Structure") (Interactor :type "/Game/Transform_Trace_interact/Blueprints/Components/BP_TraceInteractor Object Reference"))
  (returns (Return :type Boolean))
  (`self.TeleportPlayer`)
  (return false))

(fn `UserConstructionScript`
  (`parent.UserConstructionScript`)
  (`self.SetupNode`))